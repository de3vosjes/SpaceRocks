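; BP_Movement is the player pawn for PhysicsTest, handling movement, look, health and UI.
; On BeginPlay it adds the Enhanced Input context and HUD; input drives control-rotation movement, inverted-pitch look and a clamped thrust value that is only printed here.
; P opens a pause widget, and Subtract self-damages for testing.
; Damage plays an impact sound; at zero health, after a delay, it loads MainMenu as a level instance and shows its menu widget.
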(event `self.ReceiveBeginPlay`
  (`EnhancedInputSubsystemInterface.AddMappingContext` (pcsubsystem `EnhancedInputLocalPlayerSubsystem` (`GameplayStatics.GetPlayerController` 0)) "/Game/Dynamic/PhysicsTest/Input_Actions/IMC_Movement.IMC_Movement" 0 (struct))
  (bind _returnvalue (`|CreateWidget` "/Game/Dynamic/FirstPerson/HUD/Widgets/WBP_HUD.WBP_HUD_C" (`GameplayStatics.GetPlayerController` 0)))
  (`UserWidget.AddToPlayerScreen` _returnvalue 0))

(event `EnhancedInput|/Game/Dynamic/PhysicsTest/Input_Actions/IA_PlayerMove`
  (params (ActionValue :type "Vector2D Structure") (ElapsedSeconds :type "Float (double-precision)") (TriggeredSeconds :type "Float (double-precision)") (InputAction :type "InputAction Object Reference" :default "/Game/Dynamic/PhysicsTest/Input_Actions/IA_PlayerMove.IA_PlayerMove"))
  (bind (_x _y) (`KismetMathLibrary.BreakVector2D` ActionValue))
  ; WASD Movement
  (:`Triggered`
    (`self.AddMovementInput` (`KismetMathLibrary.GetRightVector` (`self.GetControlRotation`)) _x)
    (`self.AddMovementInput` (`KismetMathLibrary.GetForwardVector` (`self.GetControlRotation`)) _y)))

(event `EnhancedInput|/Game/Dynamic/PhysicsTest/Input_Actions/IA_PlayerLook`
  (params (ActionValue :type "Vector2D Structure") (ElapsedSeconds :type "Float (double-precision)") (TriggeredSeconds :type "Float (double-precision)") (InputAction :type "InputAction Object Reference" :default "/Game/Dynamic/PhysicsTest/Input_Actions/IA_PlayerLook.IA_PlayerLook"))
  (bind (_x _y) (`KismetMathLibrary.BreakVector2D` (`KismetMathLibrary.MakeVector2D` ActionValue_X ActionValue_Y)))
  (:`Triggered`
    (`self.AddControllerYawInput` _x)
    (`self.AddControllerPitchInput` (* _y -1.0))))

(event `EnhancedInput|/Game/Dynamic/PhysicsTest/Input_Actions/IA_ThrustControl`
  (params (ActionValue :type "Float (double-precision)") (ElapsedSeconds :type "Float (double-precision)") (TriggeredSeconds :type "Float (double-precision)") (InputAction :type "InputAction Object Reference" :default "/Game/Dynamic/PhysicsTest/Input_Actions/IA_ThrustControl.IA_ThrustControl"))
  (:`Triggered`
    (bind _output_get (set `self.CurrentThrust` (`KismetMathLibrary.FClamp` (+ (* ActionValue 25.0) (`self.CurrentThrust`)) (`self.MinThrust`) (`self.MaxThrust`))))
    (`KismetSystemLibrary.PrintString` (`KismetStringLibrary.Conv_DoubleToString` _output_get))))

(event `Key|P`
  (params (Key :type "Key Structure"))
  (bind _returnvalue (`GameplayStatics.GetPlayerController` 0))
  (:`Pressed`
    (bind _returnvalue_2 (`|CreateWidget` "/Game/Dynamic/FirstPerson/HUD/Widgets/WBP_Pause.WBP_Pause_C"))
    (`UserWidget.AddToPlayerScreen` _returnvalue_2 0)
    (`WidgetBlueprintLibrary.SetInputMode_UIOnlyEx` _returnvalue null)
    (set `PlayerController.bShowMouseCursor` true _returnvalue)))

(event `Key|Subtract`
  (params (Key :type "Key Structure"))
  (:`Pressed`
    (`GameplayStatics.ApplyDamage` self 10.0)))

(event `self.ReceiveAnyDamage`
  (params (Damage :type "Float (single-precision)") (DamageType :type "DamageType Object Reference") (InstigatedBy :type "Controller Object Reference") (DamageCauser :type "Actor Object Reference"))
  (bind _returnvalue (`GameplayStatics.GetPlayerController` 0))
  (set `self.Health` (- (`self.Health`) Damage))
  (if (<= (`self.Health`) 0.0)
    (`KismetSystemLibrary.PrintString` "Dead")
    (`KismetSystemLibrary.Delay` 1.0)
    (`WidgetLayoutLibrary.RemoveAllWidgets`)
    (`LevelStreamingDynamic.LoadLevelInstance` "MainMenu" (0.0 0.0 0.0) (struct) "" null)
    (bind _returnvalue_2 (`|CreateWidget` "/Game/Dynamic/MainMenu/WP_MainMenu.WP_MainMenu_C"))
    (`UserWidget.AddToPlayerScreen` _returnvalue_2 0)
    (`WidgetBlueprintLibrary.SetInputMode_UIOnlyEx` _returnvalue null)
    (set `PlayerController.bShowMouseCursor` true _returnvalue)
    (else
      (`KismetSystemLibrary.PrintString` (`KismetStringLibrary.Conv_DoubleToString` (`self.Health`)))
      (`GameplayStatics.PlaySoundAtLocation` "/Game/Static/Soundeffects/asteroid-hitting-something-152511.asteroid-hitting-something-152511" (`self.K2_GetActorLocation`) (struct) 0.3 1.0 0.0 null null null null))))

(fn `UserConstructionScript`)