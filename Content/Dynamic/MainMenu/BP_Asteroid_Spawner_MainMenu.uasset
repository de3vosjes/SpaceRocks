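; Main menu spawner actor that keeps spawning floating BP_Asteroid_float_MainMenu asteroids inside a box area.
; BeginPlay starts a looping SpawnAsteroid timer, with its random interval rolled only once.
; SpawnAsteroid offsets the root's world location by a random point in SpawnArea's unscaled extent, ignoring box scale and rotation.
; A separate StartSpawning event, noted as a test fix, spawns every second by re-calling itself, with no caller here.
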(event `StartSpawning`
  ; quick fix to test issues
  (`self.SpawnAsteroid`)
  (`KismetSystemLibrary.Delay` 1.0)
  (`self.StartSpawning`))

(event `self.ReceiveBeginPlay`
  (`KismetSystemLibrary.K2_SetTimer` null "SpawnAsteroid" (`KismetMathLibrary.RandomFloatInRange` 1.0 3.0) true))

(fn `SpawnAsteroid`
  (bind _x (.x (`BoxComponent.GetUnscaledBoxExtent` (`self.Spawn_area`))))
  (bind _y (.y (`BoxComponent.GetUnscaledBoxExtent` (`self.Spawn_area`))))
  (bind _z (.z (`BoxComponent.GetUnscaledBoxExtent` (`self.Spawn_area`))))
  ; Only spawns from middle of box or at 0,0,0(extensively tested)
  (`|SpawnActorFromClass` "/Game/Dynamic/MainMenu/BP_Asteroid_float_MainMenu.BP_Asteroid_float_MainMenu_C" (`KismetMathLibrary.MakeTransform` (+ (`KismetMathLibrary.MakeVector` (`KismetMathLibrary.RandomFloatInRange` (* _x -1.0) _x) (`KismetMathLibrary.RandomFloatInRange` (* _y -1.0) _y) (`KismetMathLibrary.RandomFloatInRange` (* _z -1.0) _z)) (`SceneComponent.K2_GetComponentLocation` (`self.DefaultSceneRoot`)))) "Undefined" "MultiplyWithRoot" null null))

(fn `UserConstructionScript`)