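; BP_Asteroid_float is a drifting physics asteroid, filed under the main menu, that explodes on impact.
; BeginPlay randomizes its per-axis scale, mass, linear and angular velocity, then picks a mesh and material from arrays, so each instance looks and moves differently.
; Any hit spawns an explosion emitter and sound at the impact point, then destroys the actor.
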(event `self.ReceiveBeginPlay`
  (bind _returnvalue (`KismetMathLibrary.RandomFloatInRange` 0.5 1.5))
  (bind _asteroidmeshes (`self.AsteroidMeshes`))
  (bind _asteroidmaterials (`self.AsteroidMaterials`))
  ; Random attributes (scale, mass, rotation, material, mesh)
  (`SceneComponent.SetWorldScale3D` (`self.AsteroidMesh`) (`KismetMathLibrary.MakeVector` _returnvalue _returnvalue _returnvalue))
  (`PrimitiveComponent.SetMassOverrideInKg` (`self.AsteroidMesh`) "None" (`KismetMathLibrary.RandomFloatInRange` 100.0 1000.0) true)
  (`PrimitiveComponent.SetPhysicsLinearVelocity` (`self.AsteroidMesh`) (* (`KismetMathLibrary.RandomFloatInRange` 50.0 800.0) (`KismetMathLibrary.RandomUnitVector`)) false "None")
  (`PrimitiveComponent.SetPhysicsAngularVelocityInDegrees` (`self.AsteroidMesh`) (* (`KismetMathLibrary.RandomUnitVector`) (`KismetMathLibrary.RandomFloatInRange` 5.0 60.0)) false "None")
  (`StaticMeshComponent.SetStaticMesh` (`self.AsteroidMesh`) (`|GetArrayItem` _asteroidmeshes (`KismetMathLibrary.RandomIntegerInRange` 0 (- (`KismetArrayLibrary.Array_Length` _asteroidmeshes) 1))))
  (`PrimitiveComponent.SetMaterial` (`self.AsteroidMesh`) 0 (`|GetArrayItem` _asteroidmaterials (`KismetMathLibrary.RandomIntegerInRange` 0 (- (`KismetArrayLibrary.Array_Length` _asteroidmaterials) 1)))))

(event `self.ReceiveHit`
  (params (MyComp :type "PrimitiveComponent Object Reference") (Other :type "Actor Object Reference") (OtherComp :type "PrimitiveComponent Object Reference") (bSelfMoved :type Boolean) (HitLocation :type "Vector Structure") (HitNormal :type "Vector Structure") (NormalImpulse :type "Vector Structure") (Hit :type "HitResult Structure (by ref)"))
  (bind (_bblockinghit _binitialoverlap _time _distance _location) (`GameplayStatics.BreakHitResult` Hit))
  (`GameplayStatics.SpawnEmitterAtLocation` "/Game/Realistic_Starter_VFX_Pack_Vol2/Particles/Explosion/P_Explosion_Side.P_Explosion_Side" _location)
  (`GameplayStatics.PlaySoundAtLocation` "/Game/Static/Soundeffects/missile-explosion.missile-explosion" _location (struct) 1.0 1.0 0.0 null null null null)
  (`self.K2_DestroyActor`))

(fn `UserConstructionScript`)